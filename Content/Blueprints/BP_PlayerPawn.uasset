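; BP_PlayerPawn is the player-controlled pawn that slides sideways and fires projectiles.
; The Move Right axis applies a swept world Y offset scaled by speed and frame time, only while the predicted position stays within a symmetric MovementRange around the world origin.
; Pressing Shoot Projectile spawns a BP_PlayerProjectile at the pawn's own transform.
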(event `InputAxis|Move Right`
  (params (AxisValue :type "Float (single-precision)"))
  (bind (_returnvalue_x _returnvalue_y) (`KismetMathLibrary.BreakVector` (`self.K2_GetActorLocation`)))
  (bind _movementrange (`self.MovementRange`))
  (bind _returnvalue (* AxisValue (`self.MovementSpeed`) (`GameplayStatics.GetWorldDeltaSeconds`)))
  (if (`KismetMathLibrary.InRange_FloatFloat` (+ _returnvalue_y _returnvalue) (* _movementrange -1.0) _movementrange)
    (`self.K2_AddActorWorldOffset` (`KismetMathLibrary.MakeVector` 0.0 _returnvalue) true)))

(event `InputAction|Shoot Projectile`
  (params (Key :type "Key Structure"))
  (:`Pressed`
    (`|SpawnActorFromClass` "/Game/Blueprints/BP_PlayerProjectile.BP_PlayerProjectile_C" (`self.GetTransform`) "Undefined" "OverrideRootScale" null null)))

(fn `UserConstructionScript`)