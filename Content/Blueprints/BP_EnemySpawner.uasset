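; Enemy wave spawner that moves a formation in a Space Invaders-style zigzag.
; SpawnLoop fills the box zone with a grid of BP_EnemyActor attached to the spawner, deriving the right travel limit from row width.
; Tick moves the whole actor via CalculateOffset, a direction state machine cycling right, down, left, down.
; An interface event counts deaths, then resets to the origin and respawns the wave after a short delay.
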(event `self.ReceiveBeginPlay`
  (set `self.Origin` (`self.K2_GetActorLocation`))
  (set `self.XOffset` (/ (`self.DistanceBetweenEnemies`) 2.0))
  (`self.Spawn Enemies` 14))

(event `Spawn Enemies`
  (params (Nb :type Integer))
  (`self.SpawnLoop` Nb))

(event `/Game/Blueprints/I_OnEnemyDestroyed.Interface_OnEnemyDestroyed`
  (bind _output_get (set `self.NbEnemies_Current` (- (`self.NbEnemies_Current`) 1)))
  (if (<= _output_get 0)
    (set `self.CanMove` false)
    (set `self.EnemyDirection` "NewEnumerator0")
    (set `self.ReversedEnumProgression` false)
    (set `self.CurrentXOffset` 0.0)
    (`self.K2_SetActorLocation` (`self.Origin`))
    (`KismetSystemLibrary.Delay` 1.0)
    (`self.Spawn Enemies` 14)
    (set `self.CanMove` true)))

(event `self.ReceiveTick`
  (params (DeltaSeconds :type "Float (single-precision)"))
  (if (`self.CanMove`)
    (`self.K2_AddActorWorldOffset` (`self.CalculateOffset`) true)))

(fn `CalculateOffset`
  (returns (Offset :type "Vector Structure"))
  (locals (Offset_Local :type "Vector Structure") (CalculatedOffset_Local :type "Float (double-precision)" :default 0.0))
  (bind (_returnvalue_x _returnvalue_y) (`KismetMathLibrary.BreakVector` (`self.K2_GetActorLocation`)))
  (bind (_returnvalue_x_2 _returnvalue_y_2) (`KismetMathLibrary.BreakVector` (`self.K2_GetActorLocation`)))
  (bind _farrightlocation (`self.FarRightLocation`))
  (bind (_origin_x _origin_y) (`KismetMathLibrary.BreakVector` (`self.Origin`)))
  (bind _xoffset (`self.XOffset`))
  (bind _currentxoffset (`self.CurrentXOffset`))
  (bind _returnvalue (+ (`local.CalculatedOffset_Local`) _currentxoffset))
  (set `local.CalculatedOffset_Local` (* (`self.Speed`) (`GameplayStatics.GetWorldDeltaSeconds`)))
  (switch `/Game/Blueprints/Enum_EnemyDirection` (`self.EnemyDirection`)
    (:`NewEnumerator0`
      (if (>= (+ (`local.CalculatedOffset_Local`) _returnvalue_y_2) _farrightlocation)
        (set `local.Offset_Local` (`KismetMathLibrary.MakeVector` 0.0 (- _farrightlocation _returnvalue_y_2)))
        (set `self.EnemyDirection` "NewEnumerator1")
        (set `self.ReversedEnumProgression` false)
        (else
          (set `local.Offset_Local` (`KismetMathLibrary.MakeVector` 0.0 (`local.CalculatedOffset_Local`)))))
      (return (`local.Offset_Local`)))
    (:`NewEnumerator1`
      (if (>= _returnvalue _xoffset)
        (set `local.Offset_Local` (`KismetMathLibrary.MakeVector` (- _xoffset _currentxoffset)))
        (set `self.CurrentXOffset` 0.0)
        (if (`self.ReversedEnumProgression`)
          (set `self.EnemyDirection` "NewEnumerator0")
          (else
            (set `self.EnemyDirection` "NewEnumerator2")))
        (else
          (set `self.CurrentXOffset` _returnvalue)
          (set `local.Offset_Local` (`KismetMathLibrary.MakeVector` (* (`local.CalculatedOffset_Local`) -1.0)))))
      (return (`local.Offset_Local`)))
    (:`NewEnumerator2`
      (if (<= (- _returnvalue_y (`local.CalculatedOffset_Local`)) _origin_y)
        (set `local.Offset_Local` (`KismetMathLibrary.MakeVector` 0.0 (- _origin_y _returnvalue_y)))
        (set `self.EnemyDirection` "NewEnumerator1")
        (set `self.ReversedEnumProgression` true)
        (else
          (set `local.Offset_Local` (`KismetMathLibrary.MakeVector` 0.0 (* (`local.CalculatedOffset_Local`) -1.0)))))
      (return (`local.Offset_Local`)))))

(fn `SpawnLoop`
  (params (Nb :type Integer))
  (locals (SpawnOrigin :type "Vector2D Structure") (NbEnemiesPerLine :type Integer) (NbEnemies :type Integer) (RightSideBoundary :type "Float (double-precision)" :default 0.0))
  (bind (_origin _boxextent) (`self.GetActorBounds` false))
  (bind (_spawnorigin_x _spawnorigin_y) (`KismetMathLibrary.BreakVector2D` (`local.SpawnOrigin`)))
  (bind _distancebetweenenemies (`self.DistanceBetweenEnemies`))
  (bind _nbenemiesperline (`local.NbEnemiesPerLine`))
  (bind (_spawnzonesize_x _spawnzonesize_y) (`KismetMathLibrary.BreakVector` (`self.SpawnZoneSize`)))
  (bind _returnvalue (`KismetMathLibrary.Conv_IntToDouble` _nbenemiesperline))
  (bind _output_get (set `self.NbEnemies_Current` Nb))
  (set `local.NbEnemies` _output_get)
  (set `local.RightSideBoundary` (+ (.y _origin) (.y _boxextent)))
  (set `local.SpawnOrigin` (`KismetMathLibrary.MakeVector2D` (+ (.x _origin) (.x _boxextent)) (- (.y _origin) (.y _boxextent))))
  (set `local.NbEnemiesPerLine` (`KismetMathLibrary.FTrunc` (/ (* _spawnzonesize_y 2.0) (`self.DistanceBetweenEnemies`))))
  (for _index (range (`local.NbEnemies`))
    (if (== (+ _index 1) _nbenemiesperline)
      (bind _returnvalue_2 (`KismetMathLibrary.Conv_IntToDouble` _index))
      (bind _returnvalue_3 (+ _spawnorigin_y (* (mod _returnvalue_2 _returnvalue) _distancebetweenenemies)))
      (set `self.FarRightLocation` (- (`local.RightSideBoundary`) _returnvalue_3)))
    (bind _returnvalue_4 (`|SpawnActorFromClass` "/Game/Blueprints/BP_EnemyActor.BP_EnemyActor_C" (`KismetMathLibrary.MakeTransform` (`KismetMathLibrary.MakeVector` (- _spawnorigin_x (* (`KismetMathLibrary.FTrunc` (/ _returnvalue_2 _returnvalue)) _distancebetweenenemies)) _returnvalue_3)) "Undefined" "OverrideRootScale" self null))
    (`self.K2_AttachToActor` _returnvalue_4 self "None" "KeepWorld" "KeepRelative" "KeepRelative" true)))

(fn `UserConstructionScript`
  (`BoxComponent.SetBoxExtent` (`self.SpawnZone`) (`self.SpawnZoneSize`) true))